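; BP_NPC is a talkable NPC that shows dialogue while the player character is inside its sphere trigger.
; It creates a W_Talk widget at BeginPlay; on overlap it registers itself as the player's NPC, shows the widget and calls NextLine.
; NextLine writes the current Dialogue entry to the text block and increments LineIndex, which is never reset here.
; Leaving the sphere removes all widgets from the screen, not just the dialogue.
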(event OnComponentBeginOverlap(Sphere)
  (params (OverlappedComponent :type Primitive%20Component%20Object%20Reference) (OtherActor :type Actor%20Object%20Reference) (OtherComp :type Primitive%20Component%20Object%20Reference) (OtherBodyIndex :type Integer) (bFromSweep :type Boolean) (SweepResult :type Hit%20Result%20Structure%20%28by%20ref%29))
  (bind _asbp_third_person_character (Utilities|Casting|CastToBP_ThirdPersonCharacter OtherActor))
  (bind _output_get (Variables|Default|SetPlayer _asbp_third_person_character))
  (Variables|/Game/ThirdPerson/Blueprints/BP_ThirdPersonCharacter.BP_ThirdPersonCharacter_C|SetNPC _output_get self)
  (Development|PrintText "HERRO!!!!")
  (UserInterface|Viewport|AddtoViewport (Variables|Default|GetW_Talk) 0)
  (CallFunction|NextLine))

(event OnComponentEndOverlap(Sphere)
  (params (OverlappedComponent :type Primitive%20Component%20Object%20Reference) (OtherActor :type Actor%20Object%20Reference) (OtherComp :type Primitive%20Component%20Object%20Reference) (OtherBodyIndex :type Integer))
  (Utilities|Casting|CastToBP_ThirdPersonCharacter OtherActor)
  (Viewport|RemoveAllWidgets))

(event Custom|Next%20Line
  (Rendering|Components|TextRender|SetText (Variables|/Game/VLamb/NPC/Widget/W_Talk.W_Talk_C|GetText_Block (Variables|Default|GetW_Talk)) (Utilities|Array|Get(acopy) (Variables|Default|GetDialogue) (Variables|Default|GetLine%20Index)))
  (Math|Integer|IncrementInt (Variables|Default|GetLine%20Index)))

(event EventBeginPlay
  (bind _returnvalue (UserInterface|CreateWidget "/Game/VLamb/NPC/Widget/W_Talk.W_Talk_C"))
  (Variables|Default|SetW_Talk _returnvalue))

(event Collision|EventActorBeginOverlap
  (params (OtherActor :type Actor%20Object%20Reference)))

(event EventTick
  (params (DeltaSeconds :type Float%20%28single-precision%29)))

(fn ConstructionScript)